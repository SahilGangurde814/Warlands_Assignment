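; BP_Basketball is a basketball actor meant to be grabbed by the VR player.
; A sphere overlap with a VRPawn stores that pawn's BallHolder and sets IsGrabable, and leaving clears both.
; Pressing GrabRight prints a debug "Hello" and attaches to BallHolder with relative transforms, without checking IsGrabable.
; No release logic is present.
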(event `self.Sphere.OnComponentBeginOverlap`
  (params (OverlappedComponent :type "PrimitiveComponent Object Reference") (OtherActor :type "Actor Object Reference") (OtherComp :type "PrimitiveComponent Object Reference") (OtherBodyIndex :type Integer) (bFromSweep :type Boolean) (SweepResult :type "HitResult Structure (by ref)"))
  (bind _asvrpawn (cast `/Game/VRTemplate/Blueprints/VRPawn` OtherActor))
  (set `self.BallHolder` (`/Game/VRTemplate/Blueprints/VRPawn.BallHolder` _asvrpawn))
  (set `self.isGrabable` true))

(event `self.Sphere.OnComponentEndOverlap`
  (params (OverlappedComponent :type "PrimitiveComponent Object Reference") (OtherActor :type "Actor Object Reference") (OtherComp :type "PrimitiveComponent Object Reference") (OtherBodyIndex :type Integer))
  (cast `/Game/VRTemplate/Blueprints/VRPawn` OtherActor)
  (set `self.BallHolder` null)
  (set `self.isGrabable` false))

(event `InputAction|GrabRight`
  (params (Key :type "Key Structure"))
  (:`Pressed`
    (`KismetSystemLibrary.PrintString` "Hello")
    (`self.K2_AttachToComponent` (`self.BallHolder`) "None" "KeepRelative" "KeepRelative" "KeepRelative")))

(fn `UserConstructionScript`)