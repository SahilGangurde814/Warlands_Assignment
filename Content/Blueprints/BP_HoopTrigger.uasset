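; BP_HoopTrigger is a basketball hoop trigger that updates the score when a BP_Basketball ends overlap with its Box component.
; With authority, it calls ServerUPdateScore on VRGameMode with true.
; On remote, it chains ServerCallClientGameMode into CallGameModeCLient, which makes the same game mode call with false.
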(event `self.Box.OnComponentEndOverlap`
  (params (OverlappedComponent :type "PrimitiveComponent Object Reference") (OtherActor :type "Actor Object Reference") (OtherComp :type "PrimitiveComponent Object Reference") (OtherBodyIndex :type Integer))
  ; Update Score
  (cast `/Game/Blueprints/BP_Basketball` OtherActor)
  (`/Engine/EditorBlueprintResources/ActorMacros.Switch Has Authority`
    (:`Authority`
      (bind _asvrgame_mode (cast `/Game/VRTemplate/Blueprints/VRGameMode` (`GameplayStatics.GetGameMode`)))
      (`/Game/VRTemplate/Blueprints/VRGameMode.ServerUPdateScore` _asvrgame_mode true))
    (:`Remote`
      (`self.ServerCallClientGameMode`))))

(event `ServerCallClientGameMode`
  (`self.callGameModeCLient`))

(event `callGameModeCLient`
  (bind _asvrgame_mode (cast `/Game/VRTemplate/Blueprints/VRGameMode` (`GameplayStatics.GetGameMode`)))
  (`/Game/VRTemplate/Blueprints/VRGameMode.ServerUPdateScore` _asvrgame_mode false))

(fn `UserConstructionScript`)