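; Player state that stores scores for two players and shows them on a floating in-world score widget.
; BeginPlay caches the actor tagged "FLoatingUI", and UpdateScoreCustom sets both scores before calling UpdateScore, which redundantly sets one by player flag.
; RepNotify functions push changes into that actor's BP_UIScore widget and print them.
; The Player 2 notify passes a literal zero instead of its stored score.
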(event `self.ReceiveBeginPlay`
  (bind _outactors (`GameplayStatics.GetAllActorsWithTag` "FLoatingUI"))
  (set `self.FloatingUI` (`|GetArrayItem` _outactors)))

(event `UpdateScoreCustom`
  (params (Player1Score :type Integer) (Player2Score :type Integer) (isPlayer1 :type Boolean))
  (bind _output_get (set `self.Player1Score` Player1Score))
  (bind _output_get_2 (set `self.Player2Score` Player2Score))
  (`self.UpdateScore` isPlayer1 _output_get _output_get_2))

(fn `OnRep_Player1Score`
  (bind _player1score (`self.Player1Score`))
  (bind _asbp_floatable_ui (cast `/Game/Blueprints/BP_FloatableUI` (`self.FloatingUI`)))
  (bind _asbp_uiscore (cast `/Game/Blueprints/BP_UIScore` (`WidgetComponent.GetUserWidgetObject` (`/Game/Blueprints/BP_FloatableUI.Widget` _asbp_floatable_ui))))
  (`/Game/Blueprints/BP_UIScore.UpdateScorePlayer1` _asbp_uiscore _player1score)
  (`KismetSystemLibrary.PrintString` (`KismetStringLibrary.Conv_IntToString` _player1score)))

(fn `OnRep_Player2Score`
  (bind _asbp_floatable_ui (cast `/Game/Blueprints/BP_FloatableUI` (`self.FloatingUI`)))
  (bind _asbp_uiscore (cast `/Game/Blueprints/BP_UIScore` (`WidgetComponent.GetUserWidgetObject` (`/Game/Blueprints/BP_FloatableUI.Widget` _asbp_floatable_ui))))
  (`/Game/Blueprints/BP_UIScore.UpdateScorePlayer2` _asbp_uiscore 0)
  (`KismetSystemLibrary.PrintString` (`KismetStringLibrary.Conv_IntToString` 0)))

(fn `UpdateScore`
  (params (isPlayer1 :type Boolean) (Player1Scoe :type Integer) (Player2Score :type Integer))
  (if isPlayer1
    (set `self.Player1Score` Player1Scoe)
    (else
      (set `self.Player2Score` Player2Score))))

(fn `UserConstructionScript`)